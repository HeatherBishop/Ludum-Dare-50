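; Level end point actor, a trolley dock that completes a ticket when the trolley vehicle arrives.
; When a PP_SampleVehicle1 overlaps its Box, it marks the vehicle unpossessed and returns control to the ThirdPersonCharacter.
; If that character's ToDoList is empty, ResetForNewTicket increments TicketsCompleted on the game mode.
; Logic to destroy the trolley and its items and respawn it at TrolleyRespawnPoint is present but disconnected.
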(event OnComponentBeginOverlap(Box)
  (params (OverlappedComponent :type Primitive%20Component%20Object%20Reference) (OtherActor :type Actor%20Object%20Reference) (OtherComp :type Primitive%20Component%20Object%20Reference) (OtherBodyIndex :type Integer) (bFromSweep :type Boolean) (SweepResult :type Hit%20Result%20Structure%20%28by%20ref%29))
  (bind _as_third_person_character (Variables|Default|GetAs%20Third%20Person%20Character))
  (bind _todolist (Variables|/Game/ThirdPersonBP/Blueprints/ThirdPersonCharacter.ThirdPersonCharacter_C|GetToDoList _as_third_person_character))
  ;[1 1 1] When Overlapped With: Posess TPC, Clear ToDoUI, Run Respawn Event IF List is empty
  (Development|PrintString (Utilities|GetDisplayName OtherActor))
  (bind _aspp_sample_vehicle_1 (Utilities|Casting|CastToPP_SampleVehicle1 OtherActor))
  (Variables|Default|SetAs%20PP%20Sample%20Vehicle%201 _aspp_sample_vehicle_1)
  (Variables|/Game/EasyVehicleSuspension/Blueprints/PP_SampleVehicle1.PP_SampleVehicle1_C|SetisPosessed _aspp_sample_vehicle_1 false)
  (Pawn|Possess (Game|GetPlayerController 0) _as_third_person_character)
  (if (<= (Utilities|Array|Length _todolist) 0)
    (Utilities|Array|Clear _todolist)
    (CallFunction|ResetforNewTicket)
    (Development|PrintString "Collided With Trolley Dock, ToDoList is empty, Restart Trolley")))

(event Custom|ResetForNewTicket
  (bind _as_third_person_game_mode (Variables|Default|GetAs%20Third%20Person%20Game%20Mode))
  ;[1 1 1] RESPAWN: Remove Items from trolley and trolley list. Respawn Trolley at RespawnPoint.
  (Variables|/Game/ThirdPersonBP/Blueprints/ThirdPersonGameMode.ThirdPersonGameMode_C|SetTicketsCompleted _as_third_person_game_mode (+ (Variables|/Game/ThirdPersonBP/Blueprints/ThirdPersonGameMode.ThirdPersonGameMode_C|GetTicketsCompleted _as_third_person_game_mode) 1)))

(event EventBeginPlay
  (bind _asthird_person_character (Utilities|Casting|CastToThirdPersonCharacter (Game|GetPlayerCharacter 0)))
  (Variables|Default|SetAs%20Third%20Person%20Character _asthird_person_character)
  (bind _asthird_person_game_mode (Utilities|Casting|CastToThirdPersonGameMode (Game|GetGameMode)))
  (Variables|Default|SetAs%20Third%20Person%20Game%20Mode _asthird_person_game_mode))

(event Collision|EventActorBeginOverlap
  (params (OtherActor :type Actor%20Object%20Reference)))

(event EventTick
  (params (DeltaSeconds :type Float%20%28single-precision%29)))

(fn ConstructionScript)