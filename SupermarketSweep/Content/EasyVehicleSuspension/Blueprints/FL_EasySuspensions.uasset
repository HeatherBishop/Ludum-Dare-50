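; Blueprint function library for the Easy Vehicle Suspension system, offering a drift measurement and bulk suspension tuning.
; GetSideMovDelta scales the right-vector dot of normalized velocity by the negated gap between planar velocity and forward-aligned velocity, yielding a signed sideways slip value.
; TweakAllActorEasySuspensions copies extension, strength, damping, parent auto-detection and precise-collision settings onto every SC_EasySuspension component of an actor.
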(fn GetSideMovDelta
  (params (smc :type Static%20Mesh%20Component%20Object%20Reference))
  (bind _returnvalue (Transformation|GetComponentVelocity smc))
  (bind _returnvalue_2 (Math|Vector|GetForwardVector smc))
  (bind _returnvalue_3 (Math|Vector|MakeVector (.x _returnvalue) (.y _returnvalue) 0.0))
  (return (* (Math|Vector|DotProduct (Math|Vector|GetRightVector smc) (Math|Vector|Normalize (Transformation|GetComponentVelocity smc))) (* (Math|Vector|VectorLength (- _returnvalue_3 (* (Math|Vector|MakeVector (.x _returnvalue_2) (.y _returnvalue_2) 0.0) (Math|Vector|VectorLength _returnvalue_3)))) -1.0))))

(fn TweakAllActorEasySuspensions
  (params (actorRef :type Actor%20Object%20Reference) (suspensionExtension :type Float%20%28single-precision%29) (suspensionStrength :type Float%20%28single-precision%29) (suspensionDamping :type Float%20%28single-precision%29) (autoDetectParentSmc :type Boolean) (preciseCollision :type Boolean))
  (for _array_element (Actor|GetComponentsByClass actorRef "/Game/EasyVehicleSuspension/Blueprints/SC_EasySuspension.SC_EasySuspension_C")
    (Variables|/Game/EasyVehicleSuspension/Blueprints/SC_EasySuspension.SC_EasySuspension_C|SetsuspensionExtension _array_element suspensionExtension)
    (Variables|/Game/EasyVehicleSuspension/Blueprints/SC_EasySuspension.SC_EasySuspension_C|SetsuspensionStrength _array_element suspensionStrength)
    (Variables|/Game/EasyVehicleSuspension/Blueprints/SC_EasySuspension.SC_EasySuspension_C|SetsuspensionDamping _array_element suspensionDamping)
    (Variables|/Game/EasyVehicleSuspension/Blueprints/SC_EasySuspension.SC_EasySuspension_C|SetautoDetectParentSmc _array_element autoDetectParentSmc)
    (Variables|/Game/EasyVehicleSuspension/Blueprints/SC_EasySuspension.SC_EasySuspension_C|SetpreciseCollision _array_element preciseCollision)))